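; BP_Controller is a player controller Blueprint that handles pausing the game and showing the pause menu.
; BeginPlay sets game-only input.
; The IA_Pause Enhanced Input action toggles pause: pausing switches to game-and-UI input, shows the cursor and adds a newly created WBP_Pause widget to the viewport.
; Unpausing restores game-only input, hides the cursor and removes that widget.
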(event `self.ReceiveBeginPlay`
  (`WidgetBlueprintLibrary.SetInputMode_GameOnly` (`GameplayStatics.GetPlayerController` 0)))

(event `EnhancedInput|/Game/Blueprints/IA_Pause`
  (params (ActionValue :type Boolean) (ElapsedSeconds :type "Float (double-precision)") (TriggeredSeconds :type "Float (double-precision)") (InputAction :type "InputAction Object Reference" :default "/Game/Blueprints/IA_Pause.IA_Pause"))
  (bind _returnvalue (`GameplayStatics.GetPlayerController` 0))
  (:`Started`
    (if (`GameplayStatics.IsGamePaused`)
      (`GameplayStatics.SetGamePaused` false)
      (`WidgetBlueprintLibrary.SetInputMode_GameOnly` _returnvalue)
      (set `self.bShowMouseCursor` false)
      (`Widget.RemoveFromParent` (stale _returnvalue_2))
      (else
        (`GameplayStatics.SetGamePaused` true)
        (`WidgetBlueprintLibrary.SetInputMode_GameAndUIEx` _returnvalue null)
        (set `self.bShowMouseCursor` true)
        (bind _returnvalue_2 (`|CreateWidget` "/Game/Blueprints/WBP_Pause.WBP_Pause_C"))
        (`UserWidget.AddToViewport` _returnvalue_2 0)))))

(fn `UserConstructionScript`)
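; BP_Damage is a hazard actor that hurts the third-person player character on contact.
; Its Box overlap event casts the other actor to BP_ThirdPersonCharacter and directly subtracts a fixed amount from its HP.
; When HP reaches zero or below, it pauses the game, shows the cursor, switches to UI-only input and displays WBP_Dead.
; Otherwise it prints a warning string.
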(event `self.Box.OnComponentBeginOverlap`
  (params (OverlappedComponent :type "PrimitiveComponent Object Reference") (OtherActor :type "Actor Object Reference") (OtherComp :type "PrimitiveComponent Object Reference") (OtherBodyIndex :type Integer) (bFromSweep :type Boolean) (SweepResult :type "HitResult Structure (by ref)"))
  (bind _returnvalue (`GameplayStatics.GetPlayerController` 0))
  (bind _asbp_third_person_character (cast `/Game/ThirdPerson/Blueprints/BP_ThirdPersonCharacter` OtherActor))
  (bind _output_get (set `/Game/ThirdPerson/Blueprints/BP_ThirdPersonCharacter.HP` (- (`/Game/ThirdPerson/Blueprints/BP_ThirdPersonCharacter.HP` _asbp_third_person_character) 50) _asbp_third_person_character))
  (if (<= _output_get 0)
    (`GameplayStatics.SetGamePaused` true)
    (set `PlayerController.bShowMouseCursor` true _returnvalue)
    (`WidgetBlueprintLibrary.SetInputMode_UIOnlyEx` _returnvalue null)
    (bind _returnvalue_2 (`|CreateWidget` "/Game/Blueprints/WBP_Dead.WBP_Dead_C"))
    (`UserWidget.AddToViewport` _returnvalue_2 0)
    (else
      (`KismetSystemLibrary.PrintString` "Dont do it again"))))

(fn `UserConstructionScript`)